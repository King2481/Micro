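; BP_Saber is a held saber weapon that deflects blaster projectiles.
; When its Hitbox begins overlapping a BP_BlasterProjectile, it plays a haptic effect on the hand holding it via the GrabComponent.
; It then sends the projectile back by setting its velocity to a reversed random direction within a cone around its forward vector, preserving speed.
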(event OnComponentBeginOverlap(Hitbox)
  (params (OverlappedComponent :type Primitive%20Component%20Object%20Reference) (OtherActor :type Actor%20Object%20Reference) (OtherComp :type Primitive%20Component%20Object%20Reference) (OtherBodyIndex :type Integer) (bFromSweep :type Boolean) (SweepResult :type Hit%20Result%20Structure%20%28by%20ref%29))
  (bind _asbp_blaster_projectile (Utilities|Casting|CastToBP_BlasterProjectile OtherActor))
  (Utilities|FlowControl|Sequence
    (:then_0
      (Class|PlayerController|PlayHapticEffect (Game|GetPlayerController 0) "/Game/Imported/VRTemplate/Haptics/PistolFireHapticEffect.PistolFireHapticEffect" (Default|GetHeldbyHand (Variables|Default|GetGrabComponent)) 1.0 false))
    (:then_1
      (Variables|/Script/Engine.MovementComponent|SetVelocity (Variables|/Script/Micro.ProjectileBase|GetProjectileMovement _asbp_blaster_projectile) (* (Math|Random|RandomUnitVectorinConeinDegrees (Transformation|GetActorForwardVector _asbp_blaster_projectile) 3e+01) -1.0 (Math|Vector|VectorLength (Variables|/Script/Engine.MovementComponent|GetVelocity (Variables|/Script/Micro.ProjectileBase|GetProjectileMovement _asbp_blaster_projectile))))))))

(event OnComponentHit(Hitbox)
  (params (HitComponent :type Primitive%20Component%20Object%20Reference) (OtherActor :type Actor%20Object%20Reference) (OtherComp :type Primitive%20Component%20Object%20Reference) (NormalImpulse :type Vector :default "0, 0, 0") (Hit :type Hit%20Result%20Structure%20%28by%20ref%29)))

(event EventBeginPlay)

(event Collision|EventActorBeginOverlap
  (params (OtherActor :type Actor%20Object%20Reference)))

(event EventTick
  (params (DeltaSeconds :type Float%20%28single-precision%29)))

(fn ConstructionScript)