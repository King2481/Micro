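; BP_Turret is a turret that fires through its BulletFiring component while moving a sphere back and forth along a spline.
; Tick eases the sphere between spline ends with FInterpTo, flipping the target on arrival.
; BeginPlay starts a delayed timer; Fire pulls the trigger and schedules another at a random interval, with the handle cleared on EndPlay.
; AimAtLocation rotates BulletFiring toward a supplied point, raised to avoid aiming at feet.
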(event EventBeginPlay
  (bind _returnvalue (Utilities|Time|SetTimerbyEvent (EventDispatchers|CreateEvent :!event Fire) 5.0 false 1e+01))
  (Variables|Default|SetFireTimerHandle _returnvalue))

(event EventTick
  (params (DeltaSeconds :type Float%20%28single-precision%29))
  (bind _output_get (Variables|Default|SetCurrent (Math|Interpolation|FInterpTo (Variables|Default|GetCurrent) (Variables|Default|GetTarget) DeltaSeconds 0.5)))
  (Transformation|SetWorldLocation (Variables|Default|GetSphere) (Spline|GetLocationatTime (Variables|Default|GetSpline) _output_get "World" true) false false)
  (if (Math|Float|NearlyEqual(Float) (Variables|Default|GetCurrent) (Variables|Default|GetTarget) 0.001)
    (Variables|Default|SetTarget (Math|Float|SelectFloat 0.0 1.0 (Math|Float|NearlyEqual(Float) (Variables|Default|GetCurrent) 1.0 0.001)))))

(event EventEndPlay
  (params (EndPlayReason :type EEndPlayReason%20Enum :default "Destroyed"))
  (Utilities|Time|ClearandInvalidateTimerbyHandle (Variables|Default|GetFireTimerHandle)))

(fn ConstructionScript)

(fn AimatLocation
  (params (LocationToAimAt :type Vector))
  (Transformation|SetWorldRotation (Variables|Default|GetBulletFiring) (Math|Rotator|FindLookatRotation (Transformation|GetWorldLocation (Variables|Default|GetBulletFiring)) (+ LocationToAimAt "0.000000,0.000000,100.000000")) false false))

(fn Fire
  (Class|BulletFiringComponent|OnPullTrigger (Variables|Default|GetBulletFiring))
  (bind _returnvalue (Utilities|Time|SetTimerbyEvent (EventDispatchers|CreateEvent :!event Fire) (Math|Random|RandomFloatinRange 3.0 6.0)))
  (Variables|Default|SetFireTimerHandle _returnvalue))