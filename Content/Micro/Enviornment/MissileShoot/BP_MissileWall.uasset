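; BP_MissileWall is a microgame hazard that fires BP_Missile projectiles from random points inside its box along the actor's forward vector.
; It enables and disables its tick through the microgame game mode's start and game-over events.
; Tick acts as the fire timer: the interval starts at five seconds, then each shot resets it from FrequencyCurve, indexed by the count of missiles fired.
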(event EventBeginPlay
  (bind _asbp_micro_game_mode_base (Utilities|Casting|CastToBP_MicroGameMode_Base (Game|GetGameMode)))
  (EventDispatchers|BindEventtoEventStartGame _asbp_micro_game_mode_base (EventDispatchers|CreateEvent :!event StartGame))
  (EventDispatchers|BindEventtoEventGameOver _asbp_micro_game_mode_base (EventDispatchers|CreateEvent :!event GameOver)))

(event EventTick
  (params (DeltaSeconds :type Float%20%28single-precision%29))
  (CallFunction|FireMissile))

(fn ConstructionScript)

(fn FireMissile
  (bind _box (Variables|Default|GetBox))
  (bind _returnvalue (Components|Box|GetUnscaledBoxExtent _box))
  (bind _returnvalue_2 (Transformation|GetWorldLocation _box))
  (bind _returnvalue_3 (Math|Random|RandomPointinBoundingBox _returnvalue_2 _returnvalue))
  (LocalVariables|SetLocalLocationChosen _returnvalue_3)
  (Class|WeaponGameplayStatics|FireProjectile self "/Game/Micro/Enviornment/MissileShoot/BP_Missile.BP_Missile_C" _returnvalue_3 (Transformation|GetActorForwardVector))
  (bind _result (Math|Integer|IncrementInt (Variables|Default|GetMissilesFired))
    (:%20%20
      (Actor|Tick|SetActorTickInterval (Math|Curves|GetFloatValue (LocalVariables|GetFrequencyCurve) (Math|Conversions|ToFloat(Integer) _result))))))

(fn GameOver
  (Actor|Tick|SetActorTickEnabled false))

(fn StartGame
  (Actor|Tick|SetActorTickEnabled true)
  (Actor|Tick|SetActorTickInterval 5.0) ; Ticks every 5 seconds.
)