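; BP_DestroyAllMissiles is a shootable pickup in the missile-shoot environment that clears all incoming missiles when hit.
; On BeginPlay it binds to its own OnTakeAnyDamage event, unbinding on EndPlay.
; Any damage plays a sound and spawns an explosion, then calls DestroyAllIncomingMissiles on its owner, assumed to always be BP_ItemWall, and destroys itself.
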(event EventBeginPlay
  (EventDispatchers|BindEventtoOnTakeAnyDamage (EventDispatchers|CreateEvent :!event OnDestroyAllHit)))

(event EventEndPlay
  (params (EndPlayReason :type EEndPlayReason%20Enum :default "Destroyed"))
  (EventDispatchers|UnbindallEventsfromOnTakeAnyDamage))

(fn ConstructionScript)

(fn OnDestroyAllHit
  (params (DamagedActor :type Actor%20Object%20Reference) (Damage :type Float%20%28single-precision%29) (DamageType :type Damage%20Type%20Object%20Reference) (InstigatedBy :type Controller%20Object%20Reference) (DamageCauser :type Actor%20Object%20Reference))
  (Audio|PlaySound2D "/Engine/VREditor/Sounds/VR_teleport_Cue.VR_teleport_Cue" 1.0 1.0 0.0 0 0)
  (Effects|SpawnEmitteratLocation "/Game/StarterContent/Particles/P_Explosion.P_Explosion" (Transformation|GetActorLocation) (Transformation|GetActorRotation))
  (bind _asbp_item_wall (Utilities|Casting|CastToBP_ItemWall (Components|GetOwner)))
  (Default|DestroyAllIncomingMissiles _asbp_item_wall)
  (Actor|DestroyActor))