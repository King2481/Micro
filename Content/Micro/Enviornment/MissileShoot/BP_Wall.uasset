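; BP_Wall is a destructible wall in the MissileShoot micro game whose destruction ends the game.
; On BeginPlay it binds to the StartGame event of BP_MicroGameMode_Base, with OnGameStart restoring full health, visibility and collision.
; When its Health component depletes, it hides itself, disables collision and calls GameOver on the game mode.
; The actor is never destroyed, so it can be reused between rounds.
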(event OnHealthDepletedDelegate(Health)
  (params (Damage :type Float%20%28single-precision%29) (DamageType :type Damage%20Type%20Object%20Reference) (InstigatedBy :type Controller%20Object%20Reference) (DamageCauser :type Actor%20Object%20Reference))
  (Rendering|SetActorHiddenInGame true)
  (Collision|SetActorEnableCollision false)
  (bind _asbp_micro_game_mode_base (Utilities|Casting|CastToBP_MicroGameMode_Base (Game|GetGameMode)))
  (Default|CallEventGameOver _asbp_micro_game_mode_base))

(event EventBeginPlay
  (bind _asbp_micro_game_mode_base (Utilities|Casting|CastToBP_MicroGameMode_Base (Game|GetGameMode)))
  (EventDispatchers|BindEventtoEventStartGame _asbp_micro_game_mode_base (EventDispatchers|CreateEvent :!event OnGameStart)))

(fn ConstructionScript)

(fn OnGameStart
  (Class|HealthComponent|SetHealthValue (Variables|Default|GetHealth) 1e+02)
  (Rendering|SetActorHiddenInGame false)
  (Collision|SetActorEnableCollision true))