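; BP_GameStarter is an actor in the MissileShoot micro game that starts a round when it takes damage.
; On any damage it calls StartGame on BP_MicroGameMode_Base, hides itself, disables its collision and resets player 0's MicroPlayerState score.
; It binds to the game mode's game-over event to show itself and re-enable collision, ready for another round.
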(event EventBeginPlay
  (EventDispatchers|BindEventtoOnTakeAnyDamage (EventDispatchers|CreateEvent :!event OnTakeDamage))
  (bind _asbp_micro_game_mode_base (Utilities|Casting|CastToBP_MicroGameMode_Base (Game|GetGameMode)))
  (EventDispatchers|BindEventtoEventGameOver _asbp_micro_game_mode_base (EventDispatchers|CreateEvent :!event OnGameOver)))

(event EventEndPlay
  (params (EndPlayReason :type EEndPlayReason%20Enum :default "Destroyed"))
  (EventDispatchers|UnbindallEventsfromOnTakeAnyDamage))

(fn ConstructionScript)

(fn OnTakeDamage
  (params (DamagedActor :type Actor%20Object%20Reference) (Damage :type Float%20%28single-precision%29) (DamageType :type Damage%20Type%20Object%20Reference) (InstigatedBy :type Controller%20Object%20Reference) (DamageCauser :type Actor%20Object%20Reference))
  (bind _asbp_micro_game_mode_base (Utilities|Casting|CastToBP_MicroGameMode_Base (Game|GetGameMode)))
  (Default|StartGame _asbp_micro_game_mode_base)
  (Rendering|SetActorHiddenInGame true)
  (Collision|SetActorEnableCollision false)
  (bind _asmicro_player_state (Utilities|Casting|CastToMicroPlayerState (Game|GetPlayerState 0)))
  (Class|MicroPlayerState|ResetScore _asmicro_player_state))

(fn OnGameOver
  (Rendering|SetActorHiddenInGame false)
  (Collision|SetActorEnableCollision true))