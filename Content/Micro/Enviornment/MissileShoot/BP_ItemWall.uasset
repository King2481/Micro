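; Item-spawning wall for the missile shoot microgame that creates pickups inside its box volume.
; While ticking, it randomly rolls for a missile-clearing item, a health pack or nothing, spawning items with itself as owner.
; It provides functions to heal the referenced wall and to damage all missiles so they explode and award points.
; Game start enables ticking; game end disables it and clears remaining missiles.
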(event EventBeginPlay
  (bind _asbp_micro_game_mode_base (Utilities|Casting|CastToBP_MicroGameMode_Base (Game|GetGameMode)))
  (EventDispatchers|BindEventtoEventStartGame _asbp_micro_game_mode_base (EventDispatchers|CreateEvent :!event GameStart))
  (EventDispatchers|BindEventtoEventGameOver _asbp_micro_game_mode_base (EventDispatchers|CreateEvent :!event GameEnd)))

(event EventTick
  (params (DeltaSeconds :type Float%20%28single-precision%29))
  (CallFunction|AttempttoSpawnItem))

(fn ConstructionScript)

(fn AttempttoSpawnItem
  (bind _box (Variables|Default|GetBox))
  (bind _output_get (LocalVariables|SetRandomInt (Math|Random|RandomIntegerinRange 1 10)))
  (switch int _output_get
    (:1
      (LocalVariables|SetItemClass "/Game/Micro/Enviornment/MissileShoot/BP_DestroyAllMissiles.BP_DestroyAllMissiles_C" :!label _label))
    (:2
      (goto _label))
    (:6
      (LocalVariables|SetItemClass "/Game/Micro/Enviornment/MissileShoot/BP_HealthPack.BP_HealthPack_C" :!label _label_2))
    (:7
      (goto _label_2))
    (:8
      (goto _label_2))
    (:9
      (goto _label_2)))
  (bind _output_get_2 (LocalVariables|SetLocalLocationChosen (Math|Random|RandomPointinBoundingBox (Transformation|GetWorldLocation _box) (Components|Box|GetScaledBoxExtent _box))))
  (Game|SpawnActorfromClass (LocalVariables|GetItemClass) (Math|Transform|MakeTransform _output_get_2 (Math|Rotator|Delta(Rotator) (Transformation|GetActorRotation) "0.000000,90.000000,0.000000")) "Undefined" self 0))

(fn RestoreHealthtoWall
  (bind _wallreference (Variables|Default|GetWallReference))
  (Utilities|IsValid _wallreference
    (:Is%20Valid
      (Class|HealthComponent|ModifyHealth (Variables|/Game/Micro/Enviornment/MissileShoot/BP_Wall.BP_Wall_C|GetHealth _wallreference) 25.0))))

(fn DestroyAllIncomingMissiles
  (bind _outactors (Actor|GetAllActorsOfClass "/Game/Micro/Enviornment/MissileShoot/BP_Missile.BP_Missile_C"))
  (for _array_element _outactors
    (Game|Damage|ApplyDamage _array_element 1.0 0 0 "/Script/Engine.DamageType") ; Apply damage so it explodes and grants points
  ))

(fn GameStart
  (Actor|Tick|SetActorTickEnabled true))

(fn GameEnd
  (Actor|Tick|SetActorTickEnabled false)
  (CallFunction|DestroyAllIncomingMissiles))